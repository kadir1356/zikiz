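; Production-band (conveyor belt) actor that carries Bp_oc actors along its forward direction.
; Every tick it queries its Box for overlapping Bp_oc actors and casts each one.
; It offsets each one's Nesne component by the forward vector scaled by Döngühizi and delta time, without sweep or physics teleport.
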(event EventTick
  (params (DeltaSeconds :type Float%20%28single-precision%29))
  (for _array_element (Collision|GetOverlappingActors (Variables|Default|GetBox) "/Game/bp/bp_oc.bp_oc_C" :!class /Script/Engine.PrimitiveComponent)
    (bind _asbp_oc (Utilities|Casting|CastTobp_oc _array_element))
    (Transformation|AddWorldOffset (Variables|/Game/bp/bp_oc.bp_oc_C|Getnesne _asbp_oc) (* (* DeltaSeconds (Variables|Default|Getdöngühizi)) (Transformation|GetActorForwardVector self)) false false)))

(fn ConstructionScript)